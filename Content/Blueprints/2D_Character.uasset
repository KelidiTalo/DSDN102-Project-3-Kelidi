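; Player-controlled Paper2D side-scroller character with run, sprint, double jump, wall slide and jump, dash and ground slide, plus a HUD.
; Tick selects the flipbook from state flags and velocity, updates jump settings, cuts slowed dashes short and traces for "WallJump"-tagged walls.
; Dash and slide set velocity along the facing direction, suspending friction and gravity until Delays restore them.
; Facing flips the character by X scale.
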(event Custom|JumpEvent
  ;[0.15 0.15 0.15 0.5] Jump Custom Event
  (if (not (Variables|Default|Getdashing))
    (Variables|Default|SetJumping true)
    (Character|Jump)
    (Utilities|FlowControl|Delay 0.8)
    (Variables|Default|SetJumping false)))

(event Custom|AnimationUpdate
  (bind _character (Variables|Default|GetCharacter))
  ;[0.15 0.15 0.15 0.5] Animation Control
  (Variables|Default|SetAnimationLogicEnum (select (Math|Boolean|ANDBoolean (< (Math|Vector|VectorLength (Variables|/Script/Engine.MovementComponent|GetVelocity (Variables|Character|GetCharacterMovement))) 1.6e+03) (not (AI|Components|NavMovement|IsFalling (Variables|Character|GetCharacterMovement))) (not (Variables|Default|Getdashing))) "NewEnumerator0" (select (Variables|Default|GetSliding) "NewEnumerator10" (select (Math|Boolean|ANDBoolean (Variables|Default|GetSlideRecovery) (== (.z (Variables|/Script/Engine.MovementComponent|GetVelocity (Variables|Character|GetCharacterMovement))) 0.0) (not (Variables|Default|Getdashing))) "NewEnumerator11" (select (Variables|Default|GetDashStart) "NewEnumerator5" (select (Variables|Default|GetDashLoop) "NewEnumerator6" (select (Variables|Default|GetDashEnd) "NewEnumerator8" (select (Math|Boolean|ANDBoolean (not (Variables|Default|GetJumping)) (Variables|Default|GetSprintAnim) (not (AI|Components|NavMovement|IsFalling (Variables|Character|GetCharacterMovement)))) "NewEnumerator2" (select (== (.z (Variables|/Script/Engine.MovementComponent|GetVelocity (Variables|Character|GetCharacterMovement))) 0.0) "NewEnumerator1" (select (and (> (.z (Variables|/Script/Engine.MovementComponent|GetVelocity (Variables|Character|GetCharacterMovement))) 0.0) (>= (Variables|Default|GetDoubleJump) 2)) "NewEnumerator9" (select (< (.z (Variables|/Script/Engine.MovementComponent|GetVelocity (Variables|Character|GetCharacterMovement))) 0.0) "NewEnumerator4" (select (and (> (.z (Variables|/Script/Engine.MovementComponent|GetVelocity (Variables|Character|GetCharacterMovement))) 0.0) (<= (Variables|Default|GetDoubleJump) 1)) "NewEnumerator3" "NewEnumerator0"))))))))))))
  (Sprite|SetFlipbook _character (Utilities|Select :Index (Variables|Default|GetAnimationLogicEnum) :NewEnumerator0 "/Game/Flipbooks/Idle_Anim.Idle_Anim" :NewEnumerator1 "/Game/Flipbooks/Run_Anim.Run_Anim" :NewEnumerator2 "/Game/Flipbooks/Sprint_Anim.Sprint_Anim" :NewEnumerator9 "/Game/Flipbooks/Double_Jump_SS1.Double_Jump_SS1" :NewEnumerator3 "/Game/Flipbooks/J_UpwardMotion.J_UpwardMotion" :NewEnumerator4 "/Game/Flipbooks/J_DownwardMotion.J_DownwardMotion" :NewEnumerator12 0 :NewEnumerator10 "/Game/Flipbooks/GroundSlide_Anim.GroundSlide_Anim" :NewEnumerator11 "/Game/Flipbooks/GroundSlideRECOVERY_ANIM.GroundSlideRECOVERY_ANIM" :NewEnumerator5 "/Game/Flipbooks/Dash_Start_Anim.Dash_Start_Anim" :NewEnumerator6 "/Game/Flipbooks/Dash_Loop_Anim.Dash_Loop_Anim" :NewEnumerator8 "/Game/Flipbooks/Dash_End_Anim.Dash_End_Anim" :NewEnumerator7 "/Game/Flipbooks/Idle_Anim.Idle_Anim"))
  (Components|Timeline|SetLooping _character (Utilities|Select :Index (Variables|Default|GetAnimationLogicEnum) :NewEnumerator0 true :NewEnumerator1 true :NewEnumerator2 true :NewEnumerator9 false :NewEnumerator3 false :NewEnumerator4 false :NewEnumerator12 false :NewEnumerator10 false :NewEnumerator11 false :NewEnumerator5 false :NewEnumerator6 true :NewEnumerator8 false :NewEnumerator7 false))
  (Audio|Components|Audio|Play _character))

(event Custom|ExitDash
  ;[0.15 0.15 0.15 0.5] Launch Input
  (Variables|Default|SetDashLoop false)
  (Variables|Default|SetDashEnd true)
  (Utilities|FlowControl|Delay 0.55)
  (Variables|Default|SetDashLoop false)
  (Variables|/Script/Engine.CharacterMovementComponent|SetGroundFriction (Variables|Character|GetCharacterMovement) 8.0)
  (Variables|/Script/Engine.CharacterMovementComponent|SetGravityScale (Variables|Character|GetCharacterMovement) 1e+01)
  (Variables|Default|SetDashEnd false)
  (Variables|Default|Setdashing false))

(event Custom|QuickExitDash
  ;[0.15 0.15 0.15 0.5] Launch Input
  (Variables|Default|SetDashLoop false)
  (Variables|/Script/Engine.CharacterMovementComponent|SetGroundFriction (Variables|Character|GetCharacterMovement) 8.0)
  (Variables|/Script/Engine.CharacterMovementComponent|SetGravityScale (Variables|Character|GetCharacterMovement) 1e+01)
  (Variables|Default|SetDashEnd false)
  (Variables|Default|Setdashing false))

(event Custom|Wall%20Slide
  (bind (_returnvalue _returnvalue2) (|LineTraceStart/Stop))
  ;[0.15 0.15 0.15 0.5] Wall Slide
  (bind _outhit (Collision|LineTraceByChannel _returnvalue _returnvalue2 "TraceTypeQuery1" false 0 "None"))
  (if (Actor|ActorHasTag (.HitActor (Collision|BreakHitResult _outhit)) "WallJump")
    (Variables|Default|SetWallSliding true)
    (|WallSlideAmount)
    (else
      (Variables|Default|SetWallSliding false))))

(event Custom|WallJump%20Event
  ;[0.15 0.15 0.15 0.5] Wall Jump event
  (Character|LaunchCharacter (* (Math|Vector|MakeVector (Variables|Default|GetFaceDirectionFloat) 0.0 1.5e+03) "-2500.000000,0.000000,2.000000") false true)
  (Variables|Default|SetFaceDirectionFloat (* (Variables|Default|GetFaceDirectionFloat) -1.0))
  (Variables|Default|SetFaceDirectionVector (* (Variables|Default|GetFaceDirectionVector) -1.0))
  (Pawn|Input|AddMovementInput (Math|Vector|MakeVector (.x (Variables|Default|GetFaceDirectionVector)) 0.0 0.0) 1.0 false)
  (Transformation|SetWorldScale3D (Variables|Default|GetCharacter) (Math|Vector|MakeVector (.x (Variables|Default|GetFaceDirectionVector)) 1.0 1.0)))

(event Custom|ExitSlide
  ;[0.15 0.15 0.15 0.5] Slide (Conditions: ONLY on the Ground, ONLY while Moving, NOT Jumping, NOT Dashing )
  (Variables|Default|SetSlideRecovery true)
  (Utilities|FlowControl|Delay 0.75)
  (Variables|Default|SetSlideRecovery false))

(event EventOnLanded
  (params (Hit :type Hit%20Result%20Structure%20%28by%20ref%29))
  ;[0.15 0.15 0.15 0.5] Jump Resetter
  (Variables|Default|SetDoubleJump 0)
  (Variables|/Script/Engine.CharacterMovementComponent|SetJumpZVelocity (Variables|Character|GetCharacterMovement) 3.7e+03))

(event EventBeginPlay
  (bind _returnvalue (UserInterface|CreateWidget "/Game/Blueprints/HUD.HUD_C"))
  (UserInterface|Viewport|AddtoViewport _returnvalue 0))

(event EventTick
  (params (DeltaSeconds :type Float%20%28single-precision%29))
  ;[0.15 0.15 0.15 0.5] Event Sequencer
  (Utilities|FlowControl|Sequence
    (:then_0
      (CallFunction|AnimationUpdate))
    (:then_1
      (CallFunction|QuickDashExit))
    (:then_2
      (CallFunction|MaxJumpCounter))
    (:then_3
      (CallFunction|DoubleJumpSetter))
    (:then_4
      (CallFunction|WallSlide))
    (:then_5)))

(event Input|ActionEvents|InputActionLaunch
  (params (Key :type Key%20Structure :default "None"))
  (bind _charactermovement (Variables|Character|GetCharacterMovement))
  ;[0.15 0.15 0.15 0.5] Launch Input
  (:Pressed
    (if (not (Variables|Default|Getdashing))
      (Variables|Default|Setdashing true)
      (Variables|/Script/Engine.MovementComponent|SetVelocity (Variables|Character|GetCharacterMovement) (Math|Vector|MakeVector (* (Variables|Default|GetFaceDirectionFloat) (Variables|Default|GetLaunchVelocity)) 0.0 0.0))
      (Variables|/Script/Engine.CharacterMovementComponent|SetGroundFriction _charactermovement 0.0)
      (Variables|/Script/Engine.CharacterMovementComponent|SetGravityScale _charactermovement 0.0)
      (Variables|Default|SetDashStart true)
      (Utilities|FlowControl|Delay 0.25)
      (Variables|Default|SetDashLoop true)
      (Variables|Default|SetDashStart false)
      (Utilities|FlowControl|Delay 0.25)
      (Variables|Default|SetDashLoop false)
      (if (Variables|Default|Getdashing)
        (CallFunction|ExitDash)))))

(event Input|ActionEvents|InputActionJump
  (params (Key :type Key%20Structure :default "None"))
  ;[0.15 0.15 0.15 0.5] Jump/Wall Jump Input
  (:Pressed
    (Math|Integer|IncrementInt (Variables|Default|GetDoubleJump)
      (:%20%20
        (if (and (not (Variables|Default|GetLaunching)) (not (Variables|Default|GetWallSliding)))
          (CallFunction|JumpEvent)
          (else
            (CallFunction|WallJumpEvent)))))))

(event Input|AxisEvents|InputAxisWalk/Run
  (params (AxisValue :type Float%20%28single-precision%29))
  ;[0.15 0.15 0.15 0.5] Walk Input
  (if (Math|Boolean|ANDBoolean (!= AxisValue 0.0) (not (Variables|Default|Getdashing)) (not (Variables|Default|GetSliding)))
    (Pawn|Input|AddMovementInput (Math|Vector|MakeVector AxisValue 0.0 0.0) 1.0 false)
    (Transformation|SetWorldScale3D (Variables|Default|GetCharacter) (Math|Vector|MakeVector AxisValue 1.0 1.0))
    (Variables|Default|SetFaceDirectionFloat AxisValue)
    (if (< AxisValue 0.0)
      (Variables|Default|SetFaceDirectionVector "-1.000000,0.000000,0.000000")
      (elif (> AxisValue 0.0)
        (Variables|Default|SetFaceDirectionVector "1.000000,0.000000,0.000000")))))

(event Input|KeyboardEvents|S
  (params (Key :type Key%20Structure :default "None"))
  (bind _charactermovement (Variables|Character|GetCharacterMovement))
  (bind _charactermovement_2 (Variables|Character|GetCharacterMovement))
  ;[0.15 0.15 0.15 0.5] Slide (Conditions: ONLY on the Ground, ONLY while Moving, NOT Jumping, NOT Dashing )
  (:Pressed
    (if (Math|Boolean|ANDBoolean (== (.z (Variables|/Script/Engine.MovementComponent|GetVelocity (Variables|Character|GetCharacterMovement))) 0.0) (>= (Math|Vector|VectorLength (Variables|/Script/Engine.MovementComponent|GetVelocity (Variables|Character|GetCharacterMovement))) 1.6e+03) (not (Variables|Default|Getdashing)) (not (Variables|Default|GetJumping)))
      (Components|Capsule|SetCapsuleHalfHeight (Variables|Collision|GetCapsuleComponent) 6e+01 true)
      (if (not (Variables|Default|GetSliding))
        (Variables|Default|SetSliding true)
        (Variables|/Script/Engine.MovementComponent|SetVelocity (Variables|Character|GetCharacterMovement) (Math|Vector|MakeVector (* (Variables|Default|GetFaceDirectionFloat) (Variables|Default|GetLaunchVelocity)) 0.0 0.0))
        (Variables|/Script/Engine.CharacterMovementComponent|SetGroundFriction _charactermovement_2 0.0)
        (Variables|/Script/Engine.CharacterMovementComponent|SetGravityScale _charactermovement_2 0.0)
        (Utilities|FlowControl|Delay 0.5)
        (Variables|/Script/Engine.CharacterMovementComponent|SetGroundFriction _charactermovement 8.0)
        (Variables|/Script/Engine.CharacterMovementComponent|SetGravityScale _charactermovement 1e+01)
        (Variables|Default|SetSliding false)
        (Components|Capsule|SetCapsuleHalfHeight (Variables|Collision|GetCapsuleComponent) 1.2e+02 true)
        (CallFunction|ExitSlide)))))

(event Input|KeyboardEvents|LeftShift
  (params (Key :type Key%20Structure :default "None"))
  (bind _charactermovement (Variables|Character|GetCharacterMovement))
  ;[0.15 0.15 0.15 0.5] Sprint input
  (:Pressed
    (CallFunction|SprintON _charactermovement))
  (:Released
    (CallFunction|SprintOFF _charactermovement)))

(fn ConstructionScript)

(fn SprintON
  (params (self2 :type Character%20Movement%20Component%20Object%20Reference))
  (Variables|/Script/Engine.CharacterMovementComponent|SetMaxWalkSpeed self2 (Variables|Default|GetSprint))
  (Variables|Default|SetSprintAnim true))

(fn SprintOFF
  (params (self2 :type Character%20Movement%20Component%20Object%20Reference))
  (Variables|/Script/Engine.CharacterMovementComponent|SetMaxWalkSpeed self2 1.6e+03)
  (Variables|Default|SetSprintAnim false))

(fn QuickDashExit
  (if (and (== (Variables|Default|Getdashing) true) (< (Math|Vector|VectorLength (Variables|/Script/Engine.MovementComponent|GetVelocity (Variables|Character|GetCharacterMovement))) (Variables|Default|GetLaunchVelocity)))
    (CallFunction|QuickExitDash)))

(fn MaxJumpCounter
  (if (AI|Components|NavMovement|IsFalling (Variables|Character|GetCharacterMovement))
    (Variables|Default|SetJumpMaxCount 2)))

(fn DoubleJumpSetter
  (if (> (Variables|Default|GetDoubleJump) 0)
    (Variables|/Script/Engine.CharacterMovementComponent|SetJumpZVelocity (Variables|Character|GetCharacterMovement) 5.1e+03)))