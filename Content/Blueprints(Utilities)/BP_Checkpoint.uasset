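; BP_Checkpoint is a checkpoint trigger that updates a 2D_Character's respawn point when the character enters its box.
; On overlap it writes its own location to the character's RespawnLocation and, through a DoOnce gate, shows a Checkpoint_Indicator widget.
; When the overlap ends, it waits briefly, removes the widget and resets the gate so the indicator can show again.
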(event OnComponentBeginOverlap(Box)
  (params (OverlappedComponent :type Primitive%20Component%20Object%20Reference) (OtherActor :type Actor%20Object%20Reference) (OtherComp :type Primitive%20Component%20Object%20Reference) (OtherBodyIndex :type Integer) (bFromSweep :type Boolean) (SweepResult :type Hit%20Result%20Structure%20%28by%20ref%29))
  (bind _as2d_character (Utilities|Casting|CastTo2D_Character OtherActor))
  (Variables|/Game/Blueprints/2D_Character.2D_Character_C|SetRespawnLocation _as2d_character (Transformation|GetActorLocation))
  (Utilities|FlowControl|DoOnce false
    (:Completed
      (bind _returnvalue (UserInterface|CreateWidget "/Game/Blueprints/Checkpoint_Indicator.Checkpoint_Indicator_C"))
      (bind _output_get (Variables|Default|SetCheckpointWidg _returnvalue))
      (UserInterface|Viewport|AddtoViewport _output_get 0))))

(event OnComponentEndOverlap(Box)
  (params (OverlappedComponent :type Primitive%20Component%20Object%20Reference) (OtherActor :type Actor%20Object%20Reference) (OtherComp :type Primitive%20Component%20Object%20Reference) (OtherBodyIndex :type Integer))
  (Utilities|Casting|CastTo2D_Character OtherActor)
  (Utilities|FlowControl|Delay 1.5)
  (Widget|RemovefromParent (Variables|Default|GetCheckpointWidg))
  (Utilities|FlowControl|DoOnce false) ; enters at Reset
)

(fn ConstructionScript)